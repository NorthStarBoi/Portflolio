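; BP_DontLook is an enemy that chases the player and triggers a jumpscare on contact.
; From BeginPlay it re-issues AI MoveTo toward the BP_Fper player character on a short repeating delay, with no line-of-sight check in this graph.
; A one-shot capsule overlap with a Player-tagged actor plays a demon sound and shows the jumpscare widget.
; After a delay it clears widgets, destroys itself and opens Lvl_ThirdPerson.
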(event `AI Move by`
  (bind _asbp_fper (cast `/Game/ThirdPerson/Blueprints/BP_Fper` (`GameplayStatics.GetPlayerCharacter` 0)))
  (set `self.FPC` _asbp_fper)
  (`AITask_MoveTo.AIMoveTo` (`AIBlueprintHelperLibrary.GetAIController` self) (0.0 0.0 0.0) (`self.FPC`) -1.0 "Disable" "Enable" true true true
    (:`then`
      (`KismetSystemLibrary.Delay` 0.2)
      (`self.AI Move by`))))

(event `self.ReceiveBeginPlay`
  (`self.AI Move by`))

(event `self.CapsuleComponent.OnComponentBeginOverlap`
  (params (OverlappedComponent :type "PrimitiveComponent Object Reference") (OtherActor :type "Actor Object Reference") (OtherComp :type "PrimitiveComponent Object Reference") (OtherBodyIndex :type Integer) (bFromSweep :type Boolean) (SweepResult :type "HitResult Structure (by ref)"))
  (if (`self.ActorHasTag` OtherActor "Player")
    (`/Engine/EditorBlueprintResources/StandardMacros.DoOnce` false
      (:`Completed`
        (`GameplayStatics.PlaySoundAtLocation` "/Game/Audio/AudioDemon.AudioDemon" (`self.K2_GetActorLocation`) (struct) 1.0 1.0 0.0 null null null null)
        (bind _returnvalue (`|CreateWidget` "/Game/UI/Widgets/Jumpscare.Jumpscare_C"))
        (`UserWidget.AddToViewport` _returnvalue 0)
        (`KismetSystemLibrary.Delay` 8.0)
        (`WidgetLayoutLibrary.RemoveAllWidgets`)
        (`self.K2_DestroyActor`)
        (`GameplayStatics.OpenLevel` "Lvl_ThirdPerson")))))

(fn `UserConstructionScript`)